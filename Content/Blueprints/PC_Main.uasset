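; PC_Main is the main player controller, handling inventory setup and the inventory screen toggle.
; On BeginPlay it reads an Android flag from the game mode and creates the UW_Inventory widget.
; It then seeds the PlayerStateMain inventory with constructed Apple InventoryItem objects, printing a message if that cast fails.
; The Inventory input shows the widget while held and removes it on release.
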(event EventBeginPlay
  ;[1 1 1] android definition task
  (bind _aspz_c_2game_mode (Utilities|Casting|CastTo (Game|GetGameMode)))
  (Variables|Default|SetIsAndroid (CallFunction|IsAndroid _aspz_c_2game_mode))
  (bind _returnvalue (UserInterface|CreateWidget "/Game/Blueprints/UW_Inventory.UW_Inventory_C" (Game|GetPlayerController 0)))
  (Variables|Default|SetInventory%20Widget _returnvalue)
  (bind _asplayer_state_main (Utilities|Casting|CastToPlayerStateMain (Variables|/Script/Engine.Controller|GetPlayerState (Game|GetPlayerController 0)))
    (:then
      (Variables|Default|SetAs%20Player%20State%20Main _asplayer_state_main)
      ;[1 1 1] Add 10 apples to inventory ( player state )
      (for _index (range 0 10)
        (bind _returnvalue_2 (Game|ConstructObjectfromClass "/Script/PZ_C_2.InventoryItem" (Utilities|GetOuterObject self)))
        (Variables|/Script/PZ_C_2.InventoryItem|SetName _returnvalue_2 "Apple")
        (Class|Inventory|AddItem (Variables|/Script/PZ_C_2.PlayerStateMain|GetInventory (Variables|Default|GetAs%20Player%20State%20Main)) _returnvalue_2)))
    (:CastFailed
      (Development|PrintString "Haha"))))

(event Input|ActionEvents|InputActionInventory
  (params (Key :type Key%20Structure))
  (:Pressed
    (UserInterface|Viewport|AddtoViewport (Variables|Default|GetInventory%20Widget) 0))
  (:Released
    (Widget|RemovefromParent (Variables|Default|GetInventory%20Widget))))

(fn ConstructionScript)