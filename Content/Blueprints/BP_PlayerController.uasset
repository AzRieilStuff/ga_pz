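; Player controller that sets up the local player's UI and routes inventory, fire and reload input.
; On BeginPlay it caches the PlayerCharacter pawn, creates the inventory and weapon stats widgets, and seeds the pawn's inventory with test apple items.
; Holding the Inventory input shows the inventory widget, while Fire and Reload forward to the pawn's weapon when valid.
; The Android platform check has empty branches.
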(event EventBeginPlay
  (Utilities|FlowControl|Sequence
    (:then_0
      ;[1 1 1] Init
      (bind _asplayer_character (Utilities|Casting|CastToPlayerCharacter (Game|Player|GetPlayerPawn 0)))
      (Variables|Default|SetPlayerPawn _asplayer_character))
    (:then_1
      ;[1 1 1] Init UI
      (bind _returnvalue (Class|Platforms|IsAndroid))
      (if _returnvalue
        _
        (else
          _))
      (bind _returnvalue_2 (UserInterface|CreateWidget "/Game/Blueprints/UI/WBP_Inventory.WBP_Inventory_C" (Game|GetPlayerController 0)))
      (Variables|Default|SetInventory%20Widget _returnvalue_2)
      (bind _returnvalue_3 (UserInterface|CreateWidget "/Game/Blueprints/UI/WBP_WeaponStats.WBP_WeaponStats_C"))
      (UserInterface|Viewport|AddtoViewport _returnvalue_3 0))
    (:then_2
      ;[1 1 1] Add 10 apples to inventory
      (for _index (range 0 10)
        (bind _returnvalue_4 (Game|ConstructObjectfromClass "/Script/PZ_C_2.InventoryItem" (Utilities|GetOuterObject self)))
        (Variables|/Script/PZ_C_2.InventoryItem|SetName _returnvalue_4 "Apple")
        (bind _returnvalue_5 (Class|PlayerCharacter|GetInventory (Variables|Default|GetPlayerPawn)))
        (Utilities|IsValid _returnvalue_5
          (:Is%20Valid
            (Class|Inventory|AddItem _returnvalue_5 _returnvalue_4))
          (:Is%20Not%20Valid
            (Development|PrintString "Inventory not loaded")))))))

(event Input|ActionEvents|InputActionInventory
  (params (Key :type Key%20Structure :default "None"))
  (:Pressed
    (UserInterface|Viewport|AddtoViewport (Variables|Default|GetInventory%20Widget) 0))
  (:Released
    (Widget|RemovefromParent (Variables|Default|GetInventory%20Widget))))

(event Input|ActionEvents|InputActionFire
  (params (Key :type Key%20Structure :default "None"))
  (bind _playerpawn (Variables|Default|GetPlayerPawn))
  (bind _weapon (Variables|/Script/PZ_C_2.BaseCharacter|GetWeapon _playerpawn))
  (:Pressed
    (if (Utilities|IsValid _weapon)
      (Class|BaseWeapon|Fire _weapon))))

(event Input|ActionEvents|InputActionReload
  (params (Key :type Key%20Structure :default "None"))
  (bind _playerpawn (Variables|Default|GetPlayerPawn))
  (bind _weapon (Variables|/Script/PZ_C_2.BaseCharacter|GetWeapon _playerpawn))
  (:Pressed
    (if (Utilities|IsValid _weapon)
      (Class|BaseWeapon|Reload _weapon))))

(fn ConstructionScript)