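; Player controller that sets up the player's Archer pawn reference and on-screen UI.
; For the local controller, BeginPlay caches the controlled pawn as Archer, shows the weapon stats and aim widgets, and pre-creates the inventory widget.
; The Inventory input adds that cached widget to the viewport while held and removes it on release.
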(event EventBeginPlay
  (bind _returnvalue (Game|GetPlayerController 0))
  (if (Pawn|IsLocalPlayerController)
    (Utilities|FlowControl|Sequence
      (:then_0
        ;[1 1 1] Init
        (bind _asarcher (Utilities|Casting|CastToArcher (Pawn|GetControlledPawn))
          (:then
            (Variables|Default|SetPlayerPawn _asarcher))
          (:CastFailed
            (Development|PrintString "Pawn check failed"))))
      (:then_1
        ;[1 1 1] Init UI
        (Utilities|FlowControl|Sequence
          (:then_0
            (bind _returnvalue_2 (UserInterface|CreateWidget "/Game/UI/WBP_WeaponStats.WBP_WeaponStats_C" _returnvalue))
            (UserInterface|Viewport|AddtoViewport _returnvalue_2 0)
            (bind _returnvalue_3 (UserInterface|CreateWidget "/Game/UI/WBP_Inventory.WBP_Inventory_C" _returnvalue))
            (Variables|Default|SetInventory%20Widget _returnvalue_3))
          (:then_1
            (bind _returnvalue_4 (UserInterface|CreateWidget "/Game/UI/WBP_Aim.WBP_Aim_C" _returnvalue))
            (UserInterface|Viewport|AddtoViewport _returnvalue_4 0)))))))

(event Input|ActionEvents|InputActionInventory
  (params (Key :type Key%20Structure :default "None"))
  (:Pressed
    (UserInterface|Viewport|AddtoViewport (Variables|Default|GetInventory%20Widget) 0))
  (:Released
    (Widget|RemovefromParent (Variables|Default|GetInventory%20Widget))))

(fn ConstructionScript)